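; Player bullet for the Runnessance game that damages StdMissile mobs on overlap or the boss through GameVars_2.
; Tick teleports it along X from its start point, climbing in Z when IsTargetBoss is set, which also disables mob hits.
; Any bullet reaching the fixed travel limit reduces boss HP and destroys itself, without a collision check.
; A damage-tiered sprite tint function exists, but its event-graph call never runs.
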(event Collision|EventActorBeginOverlap
  (params (OtherActor :type Actor%20Object%20Reference))
  (bind _asstd_missile (Utilities|Casting|CastToStdMissile OtherActor))
  (if (not (Variables|Default|GetisTargetBoss))
    (CallFunction|OnDamageMob _asstd_missile)))

(event EventTick
  (params (DeltaSeconds :type Float%20%28single-precision%29))
  (Variables|Default|SetTimeAcc (+ DeltaSeconds (Variables|Default|GetTimeAcc)))
  (bind _output_get (Variables|Default|Setloc (+ (* DeltaSeconds (Variables|Default|GetMoveSpeed)) (Variables|Default|Getloc))))
  (if (<= 9e+03 _output_get)
    (Utilities|FlowControl|DoOnce false
      (:Completed
        (CallFunction|OnDamageBoss)
        (Actor|DestroyActor)))
    (else
      (Transformation|Teleport (+ (Variables|Default|Getstartloc) (Math|Vector|MakeVector _output_get 0.0 (Math|Float|SelectFloat (+ (* (Variables|Default|GetTimeAcc) 2.5e+03) 3.0) 3.0 (Variables|Default|GetisTargetBoss)))) "0, 0, 0"))))

(fn ConstructionScript
  (Variables|Default|Setstartloc (Math|Vector|MakeVector (.X (Math|Vector|BreakVector (Variables|Default|Getstartloc))) (.Y (Math|Vector|BreakVector (Variables|Default|Getstartloc))) 0.0)))

(fn OnDamageBoss
  (bind _outactors (Actor|GetAllActorsOfClass "/Game/Runnessance/Ingame/GameVars_2.GameVars_2_C"))
  (Default|ReduceBossHP (Utilities|Array|Get(acopy) _outactors) (Variables|Default|Getdamage)))

(fn OnDamageMob
  (params (missile :type Std%20Missile%20Object%20Reference))
  (Default|DamageMe missile (Variables|Default|Getdamage))
  (Actor|DestroyActor))