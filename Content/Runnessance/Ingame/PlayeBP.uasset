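; Player vehicle Blueprint for the in-game run, rendered with Spine and auto-firing bullets.
; BeginPlay caches GameVars and RunInstance, derives move speed, then after a delay applies the chosen car skeleton and rider skin.
; Unless movement is disabled, Tick teleports laterally from GameVars position and spawns damage-stamped bullets every 0.2 game seconds, catching up missed shots.
; Helpers switch idle/turn animations without restarting, trigger the warp laser and hide vehicle parts afterward.
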(event EventBeginPlay
  (Utilities|FlowControl|Sequence
    (:then_0
      (bind _outactors (Actor|GetAllActorsOfClass "/Game/Runnessance/Ingame/GameVars_2.GameVars_2_C"))
      (Variables|Default|SetGameVars (Utilities|Array|Get(acopy) _outactors)))
    (:then_1
      (bind _asrun_instance (Utilities|Casting|CastToRunInstance (Game|GetGameInstance))
        (:then
          (bind _output_get (Variables|Default|SetRuninstance _asrun_instance))
          (Utilities|FlowControl|Sequence
            (:then_0
              (Variables|Default|SetMovespeed (* (Variables|/Game/Runnessance/MenuLevel/RunInstance.RunInstance_C|GetSpeed _output_get) (Utilities|Select :Index (Variables|/Game/Runnessance/MenuLevel/RunInstance.RunInstance_C|GetChoosedcarEnum _output_get) :NewEnumerator6 1.0 :NewEnumerator0 1.0 :NewEnumerator1 1.5 :NewEnumerator2 0.1))))))
        (:CastFailed
          (Class|VisualLoggerKismetLibrary|LogText "Game Instance Cast Failed" "Error"))))
    (:then_2
      (|GraphicSetting))))

(event EventTick
  (params (DeltaSeconds :type Float%20%28single-precision%29))
  (if (not (Variables|Default|GetMoveDisable))
    (Utilities|FlowControl|Sequence
      (:then_0
        (Utilities|MovetoPos))
      (:then_1
        (while (> (Variables|/Game/Runnessance/Ingame/GameVars_2.GameVars_2_C|GetGameTime (Variables|Default|GetGameVars)) (* (Variables|Default|GetTickCnt) 0.2))
          (Math|Integer|IncrementInt (Variables|Default|GetTickCnt)
            (:%20%20
              (bind _returnvalue (Game|SpawnActorfromClass "/Game/Runnessance/Ingame/Bullet/BulletBP.BulletBP_C" (Math|Transform|MakeTransform "9898.000000,9898.000000, 0" "0, 0,0.000000") "Undefined" 0 (Transformation|GetWorldLocation (Variables|Default|GetGunMuzzle)) (Variables|/Game/Runnessance/Ingame/GameVars_2.GameVars_2_C|GetisTargetBoss (Variables|Default|GetGameVars))))
              (Variables|/Game/Runnessance/Ingame/Bullet/BulletBP.BulletBP_C|Setdamage _returnvalue (Variables|/Game/Runnessance/MenuLevel/RunInstance.RunInstance_C|GetDamage (Variables|Default|GetRuninstance))))))))))

(event Collision|EventActorBeginOverlap
  (params (OtherActor :type Actor%20Object%20Reference)))

(fn ConstructionScript)

(fn SetIdleAnimation
  (if (not (== (Variables|Default|GetnowAnimation) 1))
    (Variables|Default|SetnowAnimation 1)
    (Class|SpineSkeletonAnimationComponent|SetAnimation (Variables|Default|GetSpineSkeletonAnimation) 0 "IDLE" true)))

(fn SetLeftAnimation
  (if (not (== (Variables|Default|GetnowAnimation) 2))
    (Variables|Default|SetnowAnimation 2)
    (Class|SpineSkeletonAnimationComponent|SetAnimation (Variables|Default|GetSpineSkeletonAnimation) 0 "TURNLEFT" true)))

(fn SetRightAnimation
  (if (not (== (Variables|Default|GetnowAnimation) 3))
    (Variables|Default|SetnowAnimation 3)
    (Class|SpineSkeletonAnimationComponent|SetAnimation (Variables|Default|GetSpineSkeletonAnimation) 0 "TURNRIGHT" true)))

(fn Warp
  (bind _aslazer_actor (Utilities|Casting|CastToLazerActor (Variables|/Script/Engine.ChildActorComponent|GetChildActor (Variables|Default|GetLzer))))
  (Components|Activation|Activate (Variables|Default|GetAudio) false)
  (Default|Display _aslazer_actor))

(fn PostWarpHide
  (Development|SetHiddeninGame (Variables|Default|GetSideCar) true true)
  (Development|SetHiddeninGame (Variables|Default|GetAddon2) true true)
  (Development|SetHiddeninGame (Variables|Default|GetAddon1) true true)
  (Development|SetHiddeninGame (Variables|Default|GetAddon3) true true)
  (Development|SetHiddeninGame (Variables|Default|GetGunMuzzle) true true)
  (Development|SetHiddeninGame (Variables|Default|GetSpineSkeletonRenderer) true true)
  (return))